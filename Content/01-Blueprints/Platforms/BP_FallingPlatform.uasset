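; BP_FallingPlatform is a platform that falls after the player steps on it and later respawns at its original place.
; It saves its starting transform on BeginPlay, and when the player overlaps its Box, it waits a set delay before enabling physics simulation on the Cube.
; After a second delay it spawns a fresh copy at the saved transform, passing on both delay settings, then destroys itself.
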(event `self.ReceiveBeginPlay`
  (set `self.DefaultTransform` (`self.GetTransform`)))

(event `self.Box.OnComponentBeginOverlap`
  (params (OverlappedComponent :type "PrimitiveComponent Object Reference") (OtherActor :type "Actor Object Reference") (OtherComp :type "PrimitiveComponent Object Reference") (OtherBodyIndex :type Integer) (bFromSweep :type Boolean) (SweepResult :type "HitResult Structure (by ref)"))
  (if (== OtherActor (`GameplayStatics.GetPlayerCharacter` 0))
    (`KismetSystemLibrary.Delay` (`self.DelayBeforeStartToFall`))
    (`PrimitiveComponent.SetSimulatePhysics` (`self.Cube`) true)
    (`KismetSystemLibrary.Delay` (`self.DelayBeforeRespawn`))
    (`|SpawnActorFromClass` "BP_FallingPlatform_C" (`self.DefaultTransform`) "Undefined" "MultiplyWithRoot" null (`self.DelayBeforeStartToFall`) (`self.DelayBeforeRespawn`) null)
    (`self.K2_DestroyActor`)))

(fn `UserConstructionScript`)